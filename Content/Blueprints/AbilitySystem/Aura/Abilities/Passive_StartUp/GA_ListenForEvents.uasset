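; Passive Gameplay Ability that turns gameplay events under the Attributes tag into attribute changes on its owner.
; On activation it waits for matching events, child tags included, and builds an EventBasedEffectClass spec for each.
; It zeroes the SetByCaller magnitude for every tag in EventTags, then overrides the received tag with the event's magnitude.
; The finished spec is applied to the owner's Ability System Component.
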(event `self.K2_ActivateAbility`
  (bind _returnvalue (`self.GetAbilitySystemComponentFromActorInfo`))
  (bind (_asynctaskproxy _payload) (`AbilityTask_WaitGameplayEvent.WaitGameplayEvent` (struct :`TagName` "Attributes") null false false)
    (:`EventReceived`
      (set `self.Spec` (`AbilitySystemComponent.MakeOutgoingSpec` _returnvalue (`self.EventBasedEffectClass`) 1.0 (`AbilitySystemComponent.MakeEffectContext` _returnvalue)))
      (for _array_element (`self.EventTags`)
        (`AbilitySystemBlueprintLibrary.AssignTagSetByCallerMagnitude` (`self.Spec`) _array_element))
      (bind (_eventtag _instigator _target _optionalobject _optionalobject2 _contexthandle _instigatortags _targettags _eventmagnitude) (break `GameplayEventData` _payload))
      (bind _returnvalue_2 (`AbilitySystemBlueprintLibrary.AssignTagSetByCallerMagnitude` (`self.Spec`) _eventtag _eventmagnitude))
      (`AbilitySystemComponent.BP_ApplyGameplayEffectSpecToSelf` (`self.GetAbilitySystemComponentFromActorInfo`) _returnvalue_2))))