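; GA_HitReact is a Gameplay Ability that plays a hit reaction montage on its avatar.
; On activation it applies GE_HitReact to the owner, then gets the montage through the avatar's CombatInterface.
; When the montage completes, is interrupted or is cancelled, it removes the effect by its stored handle and ends.
; A failed cast or missing montage only prints an error, leaving the effect applied and the ability active.
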(event `self.K2_ActivateAbility`
  (bind _returnvalue (`self.BP_ApplyGameplayEffectToOwner` "/Game/Blueprints/AbilitySystem/GameplayEffects/GE_HitReact.GE_HitReact_C"))
  (set `self.ActiveGEHitReact` _returnvalue)
  (bind _ascombat_interface (cast `CombatInterface` (`self.GetAvatarActorFromActorInfo`))
    (:`then`
      (bind _returnvalue_2 (`CombatInterface.GetHitReactMontage` _ascombat_interface))
      (`/Engine/EditorBlueprintResources/StandardMacros.IsValid` _returnvalue_2
        (:`Is Valid`
          (`AbilityTask_PlayMontageAndWait.CreatePlayMontageAndWaitProxy` "None" _returnvalue_2
            (:`OnCompleted`
              _)
            (:`OnInterrupted`
              _)
            (:`OnCancelled`
              _))
          (`self.BP_RemoveGameplayEffectFromOwnerWithHandle` (`self.ActiveGEHitReact`))
          (`self.K2_EndAbility`))
        (:`Is Not Valid`
          (`KismetSystemLibrary.PrintString` "Hit React Montage not Set" true true (struct :`R` 1.0 :`A` 1.0)))))
    (:`CastFailed`
      (`KismetSystemLibrary.PrintString` "GA_HitReact Get Avatar Actor Failed!" true true (struct :`R` 1.0 :`A` 1.0)))))